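; BP_EnemyType is an enemy that chases the player, deals contact damage and awards a score point when killed.
; Any actor overlap toggles CharacterSeen; while it is set, Tick turns the capsule toward the player and adds forward input from control yaw.
; Tick also shows health on text that faces the player.
; Hits apply damage behind a DoOnce-and-Delay cooldown, and incoming damage drains EnemyHealth until the actor is destroyed.
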(event Custom|LookEvent
  (bind _capsulecomponent (Variables|Collision|GetCapsuleComponent))
  (if (Variables|Default|GetcharacterSeen)
    (bind _asbp_first_person_character (Utilities|Casting|CastToBP_FirstPersonCharacter (Game|GetPlayerCharacter 0)))
    (Transformation|SetWorldRotation _capsulecomponent (Math|Rotator|MakeRotator (.Roll (Math|Rotator|BreakRotator (Math|Rotator|FindLookatRotation (Transformation|GetWorldLocation _capsulecomponent) (Transformation|GetActorLocation _asbp_first_person_character)))) 0.0 (.Yaw (Math|Rotator|BreakRotator (Math|Rotator|FindLookatRotation (Transformation|GetWorldLocation _capsulecomponent) (Transformation|GetActorLocation _asbp_first_person_character))))) false false)
    (Pawn|Input|AddMovementInput (Math|Vector|GetForwardVector (Math|Rotator|MakeRotator 0.0 0.0 (.yaw (Pawn|GetControlRotation :!class /Script/Engine.Pawn)))) 0.5 false)))

(event Game|Damage|EventAnyDamage
  (params (Damage :type Float%20%28single-precision%29) (DamageType :type Damage%20Type%20Object%20Reference) (InstigatedBy :type Controller%20Object%20Reference) (DamageCauser :type Actor%20Object%20Reference))
  (if (not (== InstigatedBy self))
    (Variables|Default|SetenemyHealth (- (Variables|Default|GetenemyHealth) Damage))
    (if (<= (Variables|Default|GetenemyHealth) 0.0)
      (Development|PrintString "enemy Dead")
      (bind _asbp_first_person_character (Utilities|Casting|CastToBP_FirstPersonCharacter (Game|GetPlayerCharacter 0)))
      (Variables|/Game/Dynamic/Blueprints/BP_FirstPersonCharacter.BP_FirstPersonCharacter_C|SetplayerScore _asbp_first_person_character (+ (Variables|/Game/Dynamic/Blueprints/BP_FirstPersonCharacter.BP_FirstPersonCharacter_C|GetplayerScore _asbp_first_person_character) 1))
      (Actor|DestroyActor))))

(event Collision|EventActorBeginOverlap
  (params (OtherActor :type Actor%20Object%20Reference))
  (Variables|Default|SetcharacterSeen true))

(event EventTick
  (params (DeltaSeconds :type Float%20%28single-precision%29))
  (bind _textbinder (Variables|Default|GettextBinder))
  (CallFunction|LookEvent)
  (Rendering|Components|TextRender|SetText (Variables|Default|GetEhealth) (Utilities|Text|ToText(Float) (Variables|Default|GetenemyHealth) "HalfToEven"))
  (bind _asbp_first_person_character (Utilities|Casting|CastToBP_FirstPersonCharacter (Game|GetPlayerCharacter 0)))
  (Transformation|SetWorldRotation _textbinder (Math|Rotator|FindLookatRotation (Transformation|GetWorldLocation _textbinder) (Transformation|GetActorLocation _asbp_first_person_character)) false false))

(event Collision|EventActorEndOverlap
  (params (OtherActor :type Actor%20Object%20Reference))
  (Variables|Default|SetcharacterSeen false))

(event Collision|EventHit
  (params (MyComp :type Primitive%20Component%20Object%20Reference) (Other :type Actor%20Object%20Reference) (OtherComp :type Primitive%20Component%20Object%20Reference) (bSelfMoved :type Boolean) (HitLocation :type Vector :default "0, 0, 0") (HitNormal :type Vector :default "0, 0, 0") (NormalImpulse :type Vector :default "0, 0, 0") (Hit :type Hit%20Result%20Structure%20%28by%20ref%29))
  (Utilities|FlowControl|DoOnce false :!label _label
    (:Completed
      (Game|Damage|ApplyDamage Other 1e+01 0 0)
      (Utilities|FlowControl|Delay 0.5)
      (goto _label Reset))))

(fn ConstructionScript)