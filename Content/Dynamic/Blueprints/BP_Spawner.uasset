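; Spawner actor that keeps creating AI-controlled BP_EnemyType enemies at random points and yaw inside its Box bounds, speeding up as the player's score grows.
; Tick drives a DoOnce gate that spawns, waits EnemyTimer via Delay, then resets to form the loop.
; After each wait, nested PlayerScore checks on BP_FirstPersonCharacter use one-shot DoOnce nodes to shorten EnemyTimer at three thresholds.
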(event EventTick
  (params (DeltaSeconds :type Float%20%28single-precision%29))
  (Utilities|FlowControl|DoOnce false :!label _label
    (:Completed
      (CallFunction|SpawnActor)
      (Utilities|FlowControl|Delay (Variables|Default|GetEnemy%20Timer))
      (bind _asbp_first_person_character (Utilities|Casting|CastToBP_FirstPersonCharacter (Game|GetPlayerCharacter 0)))
      (if (>= (Variables|/Game/Dynamic/Blueprints/BP_FirstPersonCharacter.BP_FirstPersonCharacter_C|GetplayerScore _asbp_first_person_character) 10)
        (Utilities|FlowControl|Sequence
          (:then_0
            (Utilities|FlowControl|DoOnce false
              (:Completed
                (Variables|Default|SetEnemy%20Timer 15.0))))
          (:then_1
            (bind _asbp_first_person_character_2 (Utilities|Casting|CastToBP_FirstPersonCharacter (Game|GetPlayerCharacter 0)))
            (if (>= (Variables|/Game/Dynamic/Blueprints/BP_FirstPersonCharacter.BP_FirstPersonCharacter_C|GetplayerScore _asbp_first_person_character_2) 20)
              (Utilities|FlowControl|Sequence
                (:then_0
                  (Utilities|FlowControl|DoOnce false
                    (:Completed
                      (Variables|Default|SetEnemy%20Timer 1e+01))))
                (:then_1
                  (bind _asbp_first_person_character_3 (Utilities|Casting|CastToBP_FirstPersonCharacter (Game|GetPlayerCharacter 0)))
                  (if (>= (Variables|/Game/Dynamic/Blueprints/BP_FirstPersonCharacter.BP_FirstPersonCharacter_C|GetplayerScore _asbp_first_person_character_3) 30)
                    (Utilities|FlowControl|DoOnce false
                      (:Completed
                        (Variables|Default|SetEnemy%20Timer 5.0))))
                  (Development|PrintString "SPAWN TIME" :!label _label_2)
                  (goto _label Reset)))
              (else
                (goto _label_2)))))
        (else
          (goto _label_2))))))

(fn ConstructionScript)

(fn SpawnActor
  (bind _box (Variables|Default|GetBox))
  (bind (_origin _boxextent) (Collision|GetComponentBounds _box))
  (bind _returnvalue (Game|SpawnActorfromClass "/Game/Dynamic/Blueprints/BP_EnemyType.BP_EnemyType_C" (Math|Transform|MakeTransform (Math|Random|RandomPointinBoundingBox _origin _boxextent) (Math|Rotator|MakeRotator 0.0 0.0 (Math|Random|RandomFloat))) "AdjustIfPossibleButDontSpawnIfColliding" "MultiplyWithRoot" 0 0))
  (Pawn|SpawnDefaultController _returnvalue))